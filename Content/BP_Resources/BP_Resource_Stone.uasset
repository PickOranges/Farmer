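; Stone resource pickup that goes into the player's backpack when touched.
; On BeginPlay it loads its data from the ResourceTable_New data table, keyed by ResourceName.
; Overlap events forward to the overlap begin/end handlers; on begin, an overlapping BP_ThirdPersonCharacter receives the data through AddToBackpackNew and the actor destroys itself.
; A TODO notes that this pickup logic belongs in Interactable.
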(event EventBeginPlay
  (bind _returnvalue (Utilities|GetDataTableRow "/Game/UI/NewUI/ResourceTable_New.ResourceTable_New" (Variables|Default|GetResourceName))
    (:then
      (bind _output_get (Variables|Default|SetResourceData _returnvalue)))))

(event Collision|EventActorEndOverlap
  (params (OtherActor :type Actor%20Object%20Reference))
  (Class|Interactable|OnActorOverlapEnd OtherActor OtherActor))

(event Collision|EventActorBeginOverlap
  (params (OtherActor :type Actor%20Object%20Reference))
  (Class|Interactable|OnActorOverlapBegin OtherActor OtherActor)
  ;[1 1 1] TODO: move this part into Interactable.
  (bind _asbp_third_person_character (Utilities|Casting|CastToBP_ThirdPersonCharacter OtherActor))
  (Default|AddtoBackpackNew _asbp_third_person_character (Variables|Default|GetResourceData))
  (Actor|DestroyActor))

(fn ConstructionScript)