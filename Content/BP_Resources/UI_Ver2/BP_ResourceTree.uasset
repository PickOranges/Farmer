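; Tree resource actor that shows an interaction prompt widget while the player character overlaps it.
; Overlap events call OnActorOverlapBegin and OnActorOverlapEnd, create UMG_InteractionE for BP_ThirdPersonCharacter, and remove any valid prompt when an overlap ends.
; The BPInteraction event is empty; disconnected logic would play the character's chopping animation if the weapon mesh is valid, but never runs.
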(event EventBPInteraction)

(event Collision|EventActorBeginOverlap
  (params (OtherActor :type Actor%20Object%20Reference))
  (Class|Interactable|OnActorOverlapBegin OtherActor OtherActor)
  (Utilities|Casting|CastToBP_ThirdPersonCharacter OtherActor)
  (bind _returnvalue (UserInterface|CreateWidget "/Game/UI/NewUI/UMG_InteractionE.UMG_InteractionE_C"))
  (UserInterface|Viewport|AddtoViewport _returnvalue 0))

(event Collision|EventActorEndOverlap
  (params (OtherActor :type Actor%20Object%20Reference))
  (Class|Interactable|OnActorOverlapEnd OtherActor OtherActor)
  (Utilities|IsValid (stale Collision|EventActorBeginOverlap _returnvalue)
    (:Is%20Valid
      (Widget|RemovefromParent (stale Collision|EventActorBeginOverlap _returnvalue)))))

(fn ConstructionScript)