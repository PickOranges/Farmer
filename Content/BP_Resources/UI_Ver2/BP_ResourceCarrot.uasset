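; Carrot resource actor that visually grows through a list of static meshes over time, starting on BeginPlay.
; A looping timer fires every few seconds to set the mesh for the current stage, debug-print the stage and increment it.
; Once the stage reaches the list length, it reapplies a hardcoded mesh index while the timer keeps running.
; A TODO questions moving the growth logic into Soil.
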(event Custom|Grow
  ;[1 1 1] TODO: How to move it into Soil?
  (Utilities|Time|SetTimerbyFunctionName 0 "ChangeMeshes" 6.0 true))

(event Custom|ChangeMeshes
  (bind _meshlist (Variables|Default|GetMeshList))
  ;[1 1 1] TODO: How to move it into Soil?
  (if (== (Variables|Default|GetStage) (Utilities|Array|Length _meshlist))
    (Components|StaticMesh|SetStaticMesh (Variables|Default|GetResourceMesh) (Utilities|Array|Get(acopy) _meshlist 2))
    (else
      (Components|StaticMesh|SetStaticMesh (Variables|Default|GetResourceMesh) (Utilities|Array|Get(acopy) _meshlist (Variables|Default|GetStage)))
      (Development|PrintString (Utilities|String|ToString(Integer) (Variables|Default|GetStage)) true true "(R=1.000000,G=0.039766,B=0.000000,A=1.000000)" 2e+01)
      (bind _result (Math|Integer|IncrementInt (Variables|Default|GetStage))
        (:%20%20
          (Variables|Default|SetStage _result))))))

(event EventBeginPlay
  ;[1 1 1] TODO: How to move it into Soil?
  (CallFunction|Grow))

(fn ConstructionScript
  (|CallParentFunction))