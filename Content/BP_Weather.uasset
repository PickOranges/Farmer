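; BP_Weather is a weather controller that switches the scene between Cloudy and Sunny looks through two events.
; Both events feed preset values into SetSkyAtomesphereParams, which sets sky atmosphere Rayleigh scattering and post-process volume exposure compensation.
; The same function creates a dynamic instance of the volumetric cloud's current material on every call, assigns it, and sets its DensityOffset parameter.
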(event Custom|Cloudy
  (CallFunction|SetSkyAtomesphereParams "(R=0.223199,G=0.260107,B=0.354167,A=1.000000)" -1.0 0.5))

(event Custom|Sunny
  (CallFunction|SetSkyAtomesphereParams "(R=0.174647,G=0.407240,B=1.000000,A=1.000000)" 0.0 0.0))

(event EventBeginPlay)

(event Collision|EventActorBeginOverlap
  (params (OtherActor :type Actor%20Object%20Reference)))

(event EventTick
  (params (DeltaSeconds :type Float%20%28single-precision%29)))

(fn ConstructionScript)

(fn SetSkyAtomesphereParams
  (params (Rayleigh%20Scattering :type Linear%20Color%20Structure) (Exposure%20Compensation :type Float%20%28single-precision%29) (Density%20Offest :type Float%20%28single-precision%29))
  (bind _volumetriccloud (Variables|Default|GetVolumetricCloud))
  (bind _volumetriccloudcomponent (Variables|/Script/Engine.VolumetricCloud|GetVolumetricCloudComponent _volumetriccloud))
  (Class|SkyAtmosphereComponent|SetRayleighScattering (Variables|/Script/Engine.SkyAtmosphere|GetSkyAtmosphereComponent (Variables|Default|GetSkyAtomsphere)) Rayleigh%20Scattering)
  (Utilities|Struct|SetmembersinPostProcessSettings (Variables|/Script/Engine.PostProcessVolume|GetSettings (Variables|Default|GetPostProcessVolume)) Exposure%20Compensation)
  (bind _returnvalue (Rendering|Material|CreateDynamicMaterialInstance (Variables|/Script/Engine.VolumetricCloudComponent|GetMaterial _volumetriccloudcomponent) "M_Cloudy" "None" :!class /Script/Engine.KismetMaterialLibrary))
  (bind _output_get (Variables|Default|SetM_Cloudy _returnvalue))
  (Rendering|Material|SetMaterial _volumetriccloudcomponent _output_get)
  (Rendering|Material|SetScalarParameterValue _output_get "DensityOffset" Density%20Offest :!class /Script/Engine.MaterialInstanceDynamic))