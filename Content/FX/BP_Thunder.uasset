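; Rain and thunderstorm actor that, when toggled on with a valid post-process volume, keeps rain above the player and strikes lightning repeatedly.
; A looping timer moves the Niagara rain, while the Thunder loop waits random intervals between strikes.
; Each strike relocates the actor ahead of the camera, picks one of two textures and animates the plane's material by Timeline.
; A brief exposure-compensation change flashes the sky before thunder plays.
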(event Custom|Strike
  (bind _thunderplane (Variables|Default|GetThunderPlane))
  (CallFunction|RandomRelocatedThunder)
  (CallFunction|RandomThunderTex)
  (bind _y (Timeline|Timeline PlayFromStart)
    (:Update
      (Rendering|Material|SetScalarParameterValueonMaterials _thunderplane "Y" _y)
      (Rendering|Material|SetScalarParameterValueonMaterials _thunderplane "Emission" (* (+ _y 1.0) 1e+01)))))

(event Custom|ToggleRain
  (bind _ns_rain (Variables|Default|GetNS_Rain))
  (if (Variables|Default|GetEnabled)
    (Components|Activation|Activate _ns_rain false)
    (Transformation|DetachFromComponent (Variables|Default|GetRainSound) "KeepRelative" "KeepRelative" "KeepRelative" true)
    ;[1 1 1] TODO: Add some collapsed Graph. If not valid, firstly add post processing volume and change it to cloudy weather.
    (Utilities|IsValid (Variables|Default|GetPostProcessingVolume)
      (:Is%20Valid
        (|Thunder)))
    (else
      (Components|Activation|Deactivate _ns_rain)
      (Variables|Default|SetEnabled false))))

(event Custom|FollowPlayer
  (Transformation|SetWorldLocation (Variables|Default|GetNS_Rain) (+ (Transformation|GetActorLocation (Game|GetPlayerCharacter 0)) "0.000000,0.000000,300.000000") false false))

(event EventBeginPlay)

(fn ConstructionScript)

(fn RandomRelocatedThunder
  (bind _returnvalue (Game|GetPlayerController 0))
  (bind _returnvalue_2 (Math|Random|RandomFloatinRange 1e+03 2e+03))
  (bind _returnvalue_3 (Game|GetPlayerCharacter 0))
  (bind _returnvalue_4 (Pawn|GetControlRotation _returnvalue :!class /Script/Engine.Controller))
  (bind _returnvalue_5 (Transformation|GetActorLocation _returnvalue_3))
  (bind _returnvalue_6 (Math|Vector|GetForwardVector _returnvalue_4))
  (bind _returnvalue_7 (* _returnvalue_6 _returnvalue_2))
  (Transformation|SetActorLocationAndRotation (+ _returnvalue_7 (* (Math|Vector|GetRightVector _returnvalue_4) (Math|Random|RandomFloatinRange -3e+03 3e+03)) _returnvalue_5 "0.000000,0.000000,500.000000") (Math|Rotator|MakeRotator 0.0 0.0 (.yaw (Math|Rotator|FindLookatRotation _returnvalue_7 _returnvalue_5)))))

(fn RandomThunderTex
  (bind _returnvalue (Rendering|Material|CreateDynamicMaterialInstance (Variables|Default|GetThunderPlane) 0 "/Game/FX/thunder_Mat.thunder_Mat" "None" :!class /Script/Engine.PrimitiveComponent))
  (Variables|Default|SetThunderMaterial _returnvalue)
  (Rendering|Material|SetTextureParameterValue _returnvalue "ThunderTex" (Utilities|Select :Index (Math|Random|RandomIntegerinRange 0 1) :Option%200 "/Game/FX/thunder.thunder" :Option%201 "/Game/FX/thunder2.thunder2")))