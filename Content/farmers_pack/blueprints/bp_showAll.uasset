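; Showcase actor in the farmers pack that flips its static mesh rapidly through the meshes of level actors tagged "tool".
; One second after BeginPlay it caches the tagged StaticMeshActors and starts a fast looping timer that calls Change by name.
; Each Change copies the indexed actor's mesh onto its component and increments the index, which never wraps back to the start.
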(event Custom|Change
  (bind _tools (Variables|Default|Gettools))
  (bind _i (Variables|Default|Geti))
  (bind _output (Utilities|Array|Get(acopy) _tools _i))
  (if (Utilities|IsValid _output)
    (Components|StaticMesh|SetStaticMesh (Variables|Default|GetStaticMesh) (Variables|/Script/Engine.StaticMeshComponent|GetStaticMesh (Variables|/Script/Engine.StaticMeshActor|GetStaticMeshComponent _output)))
    (Math|Integer|IncrementInt (Variables|Default|Geti))))

(event EventBeginPlay
  (Utilities|FlowControl|Delay 1.0)
  (bind _outactors (Actor|GetAllActorsOfClasswithTag "/Script/Engine.StaticMeshActor" "tool"))
  (Variables|Default|Settools _outactors)
  (Utilities|Time|SetTimerbyFunctionName 0 "change" 0.05 true))

(event Collision|EventActorBeginOverlap
  (params (OtherActor :type Actor%20Object%20Reference)))

(event EventTick
  (params (DeltaSeconds :type Float%20%28single-precision%29)))

(fn ConstructionScript)